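; BP_NPC is an NPC actor that loops an idle animation on its mesh from BeginPlay.
; An InteractionBox collision volume detects when a BP_ThirdPersonCharacter enters or leaves.
; The overlap events set that character's CanInteract flag and show or hide InteractIcon to match.
; The interaction itself is not handled in this Blueprint.
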(event OnComponentBeginOverlap(InteractionBox)
  (params (OverlappedComponent :type Primitive%20Component%20Object%20Reference) (OtherActor :type Actor%20Object%20Reference) (OtherComp :type Primitive%20Component%20Object%20Reference) (OtherBodyIndex :type Integer) (bFromSweep :type Boolean) (SweepResult :type Hit%20Result%20Structure%20%28by%20ref%29))
  ;[1 1 1] Allow player to interact with NPC when entering the collision box.
  (bind _asbp_third_person_character (Utilities|Casting|CastToBP_ThirdPersonCharacter OtherActor))
  (Variables|/Game/Blueprints/BP_ThirdPersonCharacter.BP_ThirdPersonCharacter_C|SetCanInteract _asbp_third_person_character true)
  (Development|SetHiddeninGame (Variables|Default|GetInteract%20Icon) false false))

(event OnComponentEndOverlap(InteractionBox)
  (params (OverlappedComponent :type Primitive%20Component%20Object%20Reference) (OtherActor :type Actor%20Object%20Reference) (OtherComp :type Primitive%20Component%20Object%20Reference) (OtherBodyIndex :type Integer))
  ;[1 1 1] Deny player from interacting with NPC when exiting the collision box.
  (bind _asbp_third_person_character (Utilities|Casting|CastToBP_ThirdPersonCharacter OtherActor))
  (Variables|/Game/Blueprints/BP_ThirdPersonCharacter.BP_ThirdPersonCharacter_C|SetCanInteract _asbp_third_person_character false)
  (Development|SetHiddeninGame (Variables|Default|GetInteract%20Icon) true false))

(event EventBeginPlay
  (Components|Animation|PlayAnimation (Variables|Character|GetMesh) "/Game/Characters/Bots/Animations/X_Idle.X_Idle" true))

(fn ConstructionScript)